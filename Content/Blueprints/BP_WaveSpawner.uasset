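; Wave spawner actor that starts the next wave of BP_Enemy when none remain in the level.
; CheckForEnemies runs on BeginPlay and calls SpawnWave if it finds no enemies; this file shows no other caller.
; SpawnWave plays a completion sound, increments CurrentWave and reads that wave's enemy count from the Waves map values by index, without a bounds check.
; Each enemy spawns at a random SpawnPositions entry, adjusted for collision where possible.
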(event `self.ReceiveBeginPlay`
  (`self.Check For Enemies`))

(event `Check For Enemies`
  (bind _outactors (`GameplayStatics.GetAllActorsOfClass` "/Game/Blueprints/BP_Enemy.BP_Enemy_C"))
  (if (== (`KismetArrayLibrary.Array_Length` _outactors) 0)
    (`self.Spawn Wave`)))

(event `Spawn Wave`
  (`GameplayStatics.PlaySound2D` "/Game/Audio/609336__kenneth_cooney__completed.609336__kenneth_cooney__completed" 1.0 1.0 0.0 null null)
  (`/Engine/EditorBlueprintResources/StandardMacros.IncrementInt` (`self.CurrentWave`)
    (:`  `
      (bind _values (`BlueprintMapLibrary.Map_Values` (`self.waves`)))
      (for _ (range 1 (+ (`|GetArrayItem` _values (- (`self.CurrentWave`) 1)) 1))
        (`|SpawnActorFromClass` "/Game/Blueprints/BP_Enemy.BP_Enemy_C" (`KismetArrayLibrary.Array_Random` (`self.SpawnPositions`)) "AdjustIfPossibleButAlwaysSpawn" "MultiplyWithRoot" null null)))))

(fn `UserConstructionScript`)