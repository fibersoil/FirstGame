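; BP_Enemy is a melee enemy character that chases the player from BeginPlay while alive.
; On reaching the player it plays a push montage, whose notify runs a debug-drawn sphere trace that damages pawns hit, then it resumes chasing.
; Incoming damage lowers health and knocks it backward, or at zero marks it dead and ragdolls the mesh.
; A looping random wander event exists but nothing starts it.
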(event `self.ReceiveBeginPlay`
  (`self.Chase Player`))

(event `wander`
  ;[0.2517 0.2517 0.2517] wander
  (`|AIMoveTo` self (`NavigationSystemV1.K2_GetRandomReachablePointInRadius` (`self.K2_GetActorLocation`) 500.0 null null) null
    (:`OnSuccess`
      (`KismetSystemLibrary.Delay` 1.0)
      (`self.wander`))))

(event `Chase Player`
  (bind _attack_trace_pos (`self.Attack Trace Pos`))
  (bind _returnvalue (`SceneComponent.K2_GetComponentLocation` _attack_trace_pos))
  ;[0.2517 0.2517 0.2517] Chase Player
  (if (`self.EnemyAlive`)
    (`|AIMoveTo` self (0.0 0.0 0.0) (`GameplayStatics.GetPlayerCharacter` 0)
      (:`OnSuccess`
        (if (`self.CanAttack`)
          (`|PlayMontage` (`self.Mesh`) "/Game/Characters/Mannequins/Animations/Manny/Push_Montage.Push_Montage"
            (:`then`
              (set `self.CanAttack` false))
            (:`OnCompleted`
              (set `self.CanAttack` true)
              (`self.Chase Player`))
            (:`OnNotifyBegin`
              (bind (_outhit _returnvalue_2) (`KismetSystemLibrary.SphereTraceSingleForObjects` :`Start` _returnvalue :`End` (+ (* (`SceneComponent.GetForwardVector` _attack_trace_pos) 100.0) _returnvalue) :`Radius` 20.0 :`ObjectTypes` (`|MakeArray` "ObjectTypeQuery3" :!type "EObjectTypeQuery Enum") :`DrawDebugType` "ForDuration"))
              (if _returnvalue_2
                (`GameplayStatics.ApplyDamage` (`.HitActor` (`GameplayStatics.BreakHitResult` _outhit)) 10.0)))))))))

(event `self.ReceiveAnyDamage`
  (params (Damage :type "Float (single-precision)") (DamageType :type "DamageType Object Reference") (InstigatedBy :type "Controller Object Reference") (DamageCauser :type "Actor Object Reference"))
  ;[0.2517 0.2517 0.2517] Damage
  (set `self.Health` (- (`self.Health`) Damage))
  (if (<= (`self.Health`) 0.0)
    (set `self.EnemyAlive` false)
    (`PrimitiveComponent.SetSimulatePhysics` (`self.Mesh`) true)
    (else
      (`self.LaunchCharacter` (+ (* (`self.GetActorForwardVector`) -200.0) (* (`self.GetActorUpVector`) 100.0))))))

(fn `UserConstructionScript`)