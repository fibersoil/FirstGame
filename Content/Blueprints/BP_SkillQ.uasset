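; BP_SkillQ is a moving skill actor that damages enemies and knocks them into the air, destroying itself after a fixed lifetime.
; Each tick it steps along MoveDirection without sweep, at a frame-rate-dependent speed.
; It also polls its Capsule for overlapping BP_Enemy actors each tick, so damage and the upward LaunchCharacter repeat every frame while overlap lasts.
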(event `self.ReceiveBeginPlay`
  (`KismetSystemLibrary.Delay` 5.0)
  (`self.K2_DestroyActor`))

(event `self.ReceiveTick`
  (params (DeltaSeconds :type "Float (single-precision)"))
  (`self.K2_SetActorLocation` (+ (`self.K2_GetActorLocation`) (* (`self.MoveDirection`) 40.0)))
  (for _array_element (`PrimitiveComponent.GetOverlappingActors` (`self.Capsule`) "/Game/Blueprints/BP_Enemy.BP_Enemy_C")
    (`GameplayStatics.ApplyDamage` _array_element 20.0)
    (bind _asbp_enemy (cast `/Game/Blueprints/BP_Enemy` _array_element))
    (`Character.LaunchCharacter` _asbp_enemy (* (`self.GetActorUpVector` _asbp_enemy) 800.0) true true)))

(fn `UserConstructionScript`)